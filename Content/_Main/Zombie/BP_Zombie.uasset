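; BP_Zombie is a melee enemy that chases the player, attacks, takes point damage and reports its death to ZombieGamemode.
; An AIMoveTo loop targeting player controller 0 retries on failure and attacks on arrival, while seeing a pawn sets walk speed.
; The attack montage's notify triggers sound and sphere-overlap damage, then chasing resumes.
; Hits reduce Health and play reactions until death stops movement, loosens collision and destroys the actor after a delay.
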(event OnSeePawn(PawnSensing)
  (params (Pawn :type Pawn%20Object%20Reference))
  ;[0.15 0.15 0.15 0.5] Chase Logic
  (Variables|/Script/Engine.CharacterMovementComponent|SetMaxWalkSpeed (Variables|Character|GetCharacterMovement) 3.6e+02))

(event Custom|ChasePlayer
  ;[0.15 0.15 0.15 0.5] Chase Logic
  (if (not (Variables|Default|GetIsDead))
    (AI|AIMoveTo self "0, 0, 0" (Game|GetPlayerController 0) 9e+01 false
      (:OnSuccess
        (CallFunction|Attack))
      (:OnFail
        (CallFunction|ChasePlayer)))))

(event Custom|Attack
  ;[0.15 0.15 0.15 0.5] Attack Logic
  (Animation|Montage|PlayMontage (Variables|Character|GetMesh) "/Game/_Main/Zombie/Animations/zombie_attack_Montage1.zombie_attack_Montage1"
    (:OnCompleted
      (CallFunction|ChasePlayer))
    (:OnNotifyBegin
      (Audio|PlaySoundatLocation "/Game/_Main/Zombie/Sounds/AttackCue.AttackCue" (Transformation|GetActorLocation) "0, 0, 0" 1.0 1.0 0.0 "/Game/MilitaryWeapSilver/Sound/Attenuation/ProjectileImpact_att.ProjectileImpact_att" 0 0 0)
      ;;[0.15 0.15 0.15 0.5] Damage To Player
      (bind (_outactors _returnvalue) (Collision|SphereOverlapActors (Transformation|GetWorldLocation (Variables|Default|GetArrow1)) 8e+01 (Utilities|Array|MakeArray "ObjectTypeQuery3") "/Game/_Main/Blueprints/BP_FirstPersonCharacter.BP_FirstPersonCharacter_C" (Utilities|Array|MakeArray self)))
      (if _returnvalue
        (for _array_element _outactors
          (Game|Damage|ApplyDamage _array_element 2e+01 (Pawn|GetController) self "/Script/Engine.DamageType"))))))

(event Custom|Death
  ;[0.15 0.15 0.15 0.5] Play Death Animation Logic
  (Variables|Default|SetIsDead true)
  (Components|Movement|StopMovementImmediately (Variables|Character|GetCharacterMovement))
  (Animation|Montage|PlayMontage (Variables|Character|GetMesh) "/Game/_Main/Zombie/Animations/zombie_dying_Montage.zombie_dying_Montage"
    (:then
      ;[0.15 0.15 0.15 0.5] Destroy Dead Zombie Body
      (Collision|SetCollisionResponsetoChannel (Variables|Collision|GetCapsuleComponent) "ECC_Pawn" "ECR_Overlap")
      (Collision|SetCollisionEnabled (Variables|Character|GetMesh) "NoCollision")
      (bind _aszombie_gamemode (Utilities|Casting|CastToZombieGamemode (Game|GetGameMode)))
      (Default|ZombieKIlled _aszombie_gamemode)
      (Utilities|FlowControl|Delay 5.0)
      (Actor|DestroyActor))))

(event EventBeginPlay
  ;[0.15 0.15 0.15 0.5] Chase Logic
  (CallFunction|ChasePlayer))

(event Game|Damage|EventPointDamage
  (params (Damage :type Float%20%28single-precision%29) (DamageType :type Damage%20Type%20Object%20Reference) (HitLocation :type Vector :default "0, 0, 0") (HitNormal :type Vector :default "0, 0, 0") (HitComponent :type Primitive%20Component%20Object%20Reference) (BoneName :type Name :default "None") (ShotFromDirection :type Vector :default "0, 0, 0") (InstigatedBy :type Controller%20Object%20Reference) (DamageCauser :type Actor%20Object%20Reference) (HitInfo :type Hit%20Result%20Structure%20%28by%20ref%29))
  ;[0.15 0.15 0.15 0.5] Health and Death Logic
  (if (not (Variables|Default|GetIsDead))
    (if (<= (Variables|Default|GetHealth) 0.0)
      (CallFunction|Death)
      (else
        (bind _output_get (Variables|Default|SetHealth (- (Variables|Default|GetHealth) Damage)))
        (Development|PrintString (Utilities|String|ToString(Float) _output_get))
        (if (<= _output_get 0.0)
          (CallFunction|Death)
          (else
            ;;[0.15 0.15 0.15 0.5] Hit Reaction
            (Animation|Montage|PlayMontage (Variables|Character|GetMesh) "/Game/_Main/Zombie/Animations/Zombie_Reaction_Hit_Montage.Zombie_Reaction_Hit_Montage")))))))

(fn ConstructionScript)