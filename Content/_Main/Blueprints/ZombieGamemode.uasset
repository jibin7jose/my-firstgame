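; Game mode for a wave-based zombie shooter that runs waves from start until the player wins.
; Each wave drops an ammo crate at a random preset location and spawns four zombies per wave number, split between two spawn points.
; A kill event counts down remaining zombies; at zero it shows the next wave's UI through the player character and spawns after a delay, or shows the win UI after the final wave.
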(event Custom|StartGame
  ;[0.15 0.15 0.15 0.5] Start Game
  (CallFunction|SpawnZombie))

(event Custom|SpawnZombie
  ;[0.15 0.15 0.15 0.5] ZombieSpawn
  (CallFunction|SpawnAmmo)
  (bind _output_get (Variables|Default|SetZombieTotal (* (Variables|Default|GetCurrentWave) 4)))
  (Variables|Default|SetZombiesLeft _output_get)
  (bind _index (Utilities|FlowControl|ForLoopwithBreak 0 _output_get :!label _label)
    (:LoopBody
      (if (== _index (/ (Variables|Default|GetZombieTotal) 2))
        (goto _label Break)
        (else
          (Game|SpawnActorfromClass "/Game/_Main/Zombie/BP_Zombie.BP_Zombie_C" (Variables|Default|GetSpawn%20Location1) "Undefined" "MultiplyWithRoot" 0 0))))
    (:Completed
      (Utilities|FlowControl|ForLoopwithBreak 1 (/ (Variables|Default|GetZombieTotal) 2)
        (:LoopBody
          (Game|SpawnActorfromClass "/Game/_Main/Zombie/BP_Zombie.BP_Zombie_C" (Variables|Default|GetSpawn%20Location2) "Undefined" "MultiplyWithRoot" 0 0))))))

(event Custom|ZombieKIlled
  ;[0.15 0.15 0.15 0.5] Wave Progression
  (bind _result (Math|Integer|DecrementInt (Variables|Default|GetZombiesLeft))
    (:%20%20
      (if (== _result 0)
        (CallFunction|WaveIncrement)))))

(event Custom|Wave%20Increment
  ;[0.15 0.15 0.15 0.5] Wave Progression
  (if (== (Variables|Default|GetCurrentWave) (Variables|Default|GetMaxWaves))
    (CallFunction|PlayerWins)
    (else
      (Math|Integer|IncrementInt (Variables|Default|GetCurrentWave)
        (:%20%20
          (CallFunction|WaveStart))))))

(event Custom|WaveStart
  ;[0.15 0.15 0.15 0.5] Start Next Wave
  (bind _asbp_first_person_character (Utilities|Casting|CastToBP_FirstPersonCharacter (Game|GetPlayerCharacter 0)))
  (Default|ShowWaveUI _asbp_first_person_character (Variables|Default|GetCurrentWave))
  (Utilities|FlowControl|Delay 5.0)
  (CallFunction|SpawnZombie))

(event Custom|Player%20Wins
  ;[0.15 0.15 0.15 0.5] Show Win Window UI
  (bind _asbp_first_person_character (Utilities|Casting|CastToBP_FirstPersonCharacter (Game|GetPlayerCharacter 0)))
  (Default|ShowWinUI _asbp_first_person_character))

(event Custom|SpawnAmmo
  ;[0.15 0.15 0.15 0.5] Spawn Ammo Crate
  (Game|SpawnActorfromClass "/Game/_Main/Blueprints/BP_AmmoCrate.BP_AmmoCrate_C" (Math|Transform|MakeTransform (Utilities|Array|Get(acopy) (Variables|Default|GetAmmoCrateLocations) (Math|Random|RandomInteger 3)) "0, 0, 0" "1.000000,1.000000,1.000000") "Undefined" "MultiplyWithRoot" 0 0))

(event EventBeginPlay
  ;[0.15 0.15 0.15 0.5] Start Game
  (CallFunction|StartGame))

(fn ConstructionScript)